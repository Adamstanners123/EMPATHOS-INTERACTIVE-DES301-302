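; A water plane actor, named as a VR variant, that provides an ocean surface with adjustable size and look.
; The construction script creates a dynamic instance of the ocean material on the surface mesh and scales the mesh in X and Y.
; It then pushes the exposed scale, variation, wave speed and two color settings into that material.
; The event graph holds only disabled stubs, so the Blueprint runs no gameplay logic.
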(event EventBeginPlay)

(event Collision|EventActorBeginOverlap
  (params (OtherActor :type Actor%20Object%20Reference)))

(event EventTick
  (params (DeltaSeconds :type Float%20%28single-precision%29)))

(fn ConstructionScript
  (bind _water_material (Variables|Default|GetWater%20Material))
  (|InitialWaterCreation_2_2)
  (Rendering|Material|SetScalarParameterValue _water_material "Water Scale" (Variables|Default|GetOverall%20Water%20Scale) :!class /Script/Engine.MaterialInstanceDynamic)
  (Rendering|Material|SetScalarParameterValue _water_material "Variation Amount" (Variables|Default|GetVariation%20Amount) :!class /Script/Engine.MaterialInstanceDynamic)
  (Rendering|Material|SetScalarParameterValue _water_material "Wave Speed" (Variables|Default|GetWave%20Speed) :!class /Script/Engine.MaterialInstanceDynamic)
  (Rendering|Material|SetVectorParameterValue _water_material "WaterColor A" (Variables|Default|GetPrimary%20Water%20Color) :!class /Script/Engine.MaterialInstanceDynamic)
  (Rendering|Material|SetVectorParameterValue _water_material "WaterColor B" (Variables|Default|GetSecondary%20Water%20Color) :!class /Script/Engine.MaterialInstanceDynamic))